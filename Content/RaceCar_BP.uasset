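; Race car actor that links to a race track spline and handles crashing, level restart and quitting.
; On BeginPlay it reads track info from the spline and snaps a crash camera to Box1, whose rotation the camera copies every tick.
; Crash, also triggered by the C key, turns the mesh into a ragdoll-profile physics body, switches the view to the crash camera and zeroes speed and acceleration.
; R reloads RacingWorld and Escape quits.
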(event `self.ReceiveBeginPlay`
  (bind _output_get (set `self.RaceTrack` (`/Game/RaceTrack.Spline` (`self.RaceTrack_BP`))))
  (`/Engine/EditorBlueprintResources/StandardMacros.IsValid` _output_get
    (:`Is Valid`
      (`self.getTrackInfo`)
      (`self.K2_AttachToComponent` (`self.CrashCamera`) (`self.Box1`) "None" "SnapToTarget" "SnapToTarget" "SnapToTarget" false))))

(event `self.ReceiveTick`
  (params (DeltaSeconds :type "Float (single-precision)"))
  (`self.K2_SetActorRotation` (`self.CrashCamera`) (`SceneComponent.K2_GetComponentRotation` (`self.Box1`)) false))

(event `self.crash`
  (bind _staticmesh (`self.StaticMesh`))
  (`PrimitiveComponent.SetCollisionProfileName` _staticmesh "Ragdoll" :!label _label)
  (`PrimitiveComponent.SetSimulatePhysics` _staticmesh true)
  (`PlayerController.SetViewTargetWithBlend` (`GameplayStatics.GetPlayerController` 0) (`self.CrashCamera`) 0.0 "VTBlend_Linear" 0.0 false)
  (set `self.currentSpeed` 0.0)
  (set `self.acceleration` 0.0))

(event `Key|C`
  (params (Key :type "Key Structure"))
  (:`Pressed`
    (goto _label)))

(event `Key|R`
  (params (Key :type "Key Structure"))
  (:`Pressed`
    (`GameplayStatics.OpenLevel` "RacingWorld")))

(event `Key|Escape`
  (params (Key :type "Key Structure"))
  (:`Pressed`
    (`KismetSystemLibrary.QuitGame` null "Quit")))

(fn `UserConstructionScript`)